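; Enemy NPC Blueprint that takes projectile damage, shows its health on a widget and handles its own death.
; BeginPlay and each ProyectilHit event push the normalized health ratio to the WBP_EnemyHealth widget.
; When health is depleted, it stops the AI controller's brain logic, plays a death animation alongside a 2D bell sound, then destroys the actor after a short delay.
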(event Custom|ProyectilHit
  (params (Damage :type Integer))
  (bind _output_get (Variables|Default|SetHealth (- (Variables|Default|GetHealth) Damage)))
  (bind _aswbp_enemy_health (Utilities|Casting|CastToWBP_EnemyHealth (UserInterface|GetUserWidgetObject (Variables|Default|GetEnemyHealthWidget))))
  (Default|UpdateHealth _aswbp_enemy_health (/ (Variables|Default|GetHealth) (Variables|Default|GetMaxHealth)))
  (if (<= _output_get 0.0)
    (bind _asaicontroller (Utilities|Casting|CastToAIController (Pawn|GetController)))
    (AI|Logic|StopLogic (Variables|/Script/AIModule.AIController|GetBrainComponent _asaicontroller) "")
    (Utilities|FlowControl|Sequence
      (:then_0
        (Components|Animation|PlayAnimation (Variables|Character|GetMesh) "/Game/DSDeath/Death.Death" false)
        (Utilities|FlowControl|Delay 4.0)
        (Actor|DestroyActor))
      (:then_1
        (Audio|PlaySound2D "/Game/DSDeath/Audio/darkbell.darkbell" 1.0 1.0 0.0 0 0)))))

(event EventBeginPlay
  (bind _aswbp_enemy_health (Utilities|Casting|CastToWBP_EnemyHealth (UserInterface|GetUserWidgetObject (Variables|Default|GetEnemyHealthWidget))))
  (Default|UpdateHealth _aswbp_enemy_health (/ (Variables|Default|GetHealth) (Variables|Default|GetMaxHealth))))

(fn ConstructionScript)