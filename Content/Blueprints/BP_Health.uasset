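; BP_Health is a healing zone that restores the first-person player's health while they stand inside its Box trigger.
; On overlap it stores the BP_FirstPersonCharacter and sets a Detected flag, then repeatedly adds a fixed amount to VidaActual through a short Delay loop.
; The loop ends when VidaActual reaches VidaTotal or end overlap clears the flag; the addition is unclamped, so health can overshoot the maximum.
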(event OnComponentEndOverlap(Box)
  (params (OverlappedComponent :type Primitive%20Component%20Object%20Reference) (OtherActor :type Actor%20Object%20Reference) (OtherComp :type Primitive%20Component%20Object%20Reference) (OtherBodyIndex :type Integer))
  (Utilities|Casting|CastToBP_FirstPersonCharacter OtherActor)
  (Variables|Default|SetDetected false))

(event OnComponentBeginOverlap(Box)
  (params (OverlappedComponent :type Primitive%20Component%20Object%20Reference) (OtherActor :type Actor%20Object%20Reference) (OtherComp :type Primitive%20Component%20Object%20Reference) (OtherBodyIndex :type Integer) (bFromSweep :type Boolean) (SweepResult :type Hit%20Result%20Structure%20%28by%20ref%29))
  (bind _asbp_first_person_character (Utilities|Casting|CastToBP_FirstPersonCharacter OtherActor))
  (Variables|Default|SetBP_First_Person%20Character _asbp_first_person_character)
  (Variables|Default|SetDetected true)
  (if (and (< (Variables|/Game/FirstPerson/Blueprints/BP_FirstPersonCharacter.BP_FirstPersonCharacter_C|GetVidaActual (Variables|Default|GetBP_First_Person%20Character)) (Variables|/Game/FirstPerson/Blueprints/BP_FirstPersonCharacter.BP_FirstPersonCharacter_C|GetVidaTotal (Variables|Default|GetBP_First_Person%20Character))) (Variables|Default|GetDetected)) :!label _label
    (Variables|/Game/FirstPerson/Blueprints/BP_FirstPersonCharacter.BP_FirstPersonCharacter_C|SetVidaActual (Variables|Default|GetBP_First_Person%20Character) (+ (Variables|/Game/FirstPerson/Blueprints/BP_FirstPersonCharacter.BP_FirstPersonCharacter_C|GetVidaActual (Variables|Default|GetBP_First_Person%20Character)) 5e+01))
    (Utilities|FlowControl|Delay 0.2)
    (goto _label)))

(event EventBeginPlay)

(event Collision|EventActorBeginOverlap
  (params (OtherActor :type Actor%20Object%20Reference)))

(event EventTick
  (params (DeltaSeconds :type Float%20%28single-precision%29)))

(fn ConstructionScript)