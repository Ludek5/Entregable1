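; BP_WinningBox is a level-exit trigger that sends the player to Level2 when an actor tagged Player overlaps its box.
; The overlap calls a Won event that plays a sound, prints a win message and starts a held camera fade.
; After a short delay it copies the first-person character's coins into BP_GameInstance so they persist, then opens the next level.
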(event OnComponentBeginOverlap(Box)
  (params (OverlappedComponent :type Primitive%20Component%20Object%20Reference) (OtherActor :type Actor%20Object%20Reference) (OtherComp :type Primitive%20Component%20Object%20Reference) (OtherBodyIndex :type Integer) (bFromSweep :type Boolean) (SweepResult :type Hit%20Result%20Structure%20%28by%20ref%29))
  (if (Actor|ActorHasTag OtherActor "Player")
    (CallFunction|Won)))

(event Custom|Won
  (Audio|PlaySoundatLocation 0 (Transformation|GetActorLocation) "0, 0, 0" 1.0 1.0 0.0 0 0 0 0)
  (Development|PrintString "GANASTE")
  (CameraFades|StartCameraFade :self (Game|GetPlayerCameraManager 0) :ToAlpha 3.0 :Duration 3.0 :bHoldWhenFinished true)
  (Utilities|FlowControl|Delay 0.5)
  (bind _asbp_first_person_character (Utilities|Casting|CastToBP_FirstPersonCharacter (Game|GetPlayerCharacter 0)))
  (bind _asbp_game_instance (Utilities|Casting|CastToBP_GameInstance (Game|GetGameInstance)))
  (Variables|/Game/Blueprints/BP_GameInstance.BP_GameInstance_C|SetCoins _asbp_game_instance (Variables|/Game/FirstPerson/Blueprints/BP_FirstPersonCharacter.BP_FirstPersonCharacter_C|GetCoins _asbp_first_person_character))
  (Game|OpenLevel(byName) "Level2"))

(event EventBeginPlay)

(event Collision|EventActorBeginOverlap
  (params (OtherActor :type Actor%20Object%20Reference)))

(event EventTick
  (params (DeltaSeconds :type Float%20%28single-precision%29)))

(fn ConstructionScript)