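; BP_Door is a door that opens once every coin in the level has been collected.
; On BeginPlay it counts all BP_Coin actors into RemainingCollectables and opens immediately if there are none.
; Each ItemCollected event decrements the count and calls OpenDoor at zero, which simply destroys the door actor.
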(event Custom|OpenDoor
  (Actor|DestroyActor))

(event Custom|ItemCollected
  (bind _result (Math|Integer|DecrementInt (Variables|Default|GetRemainingCollectables))
    (:%20%20
      (if (== _result 0)
        (CallFunction|OpenDoor)))))

(event EventBeginPlay
  (bind _outactors (Actor|GetAllActorsOfClass "/Game/Blueprints/BP_Coin.BP_Coin_C"))
  (bind _output_get (Variables|Default|SetRemainingCollectables (Utilities|Array|Length _outactors)))
  (if (== _output_get 0)
    (CallFunction|OpenDoor)))

(fn ConstructionScript)